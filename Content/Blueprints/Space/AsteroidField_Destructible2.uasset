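; Actor that scatters a field of randomly placed, rotated and scaled destructible asteroids in a spherical shell around itself.
; The construction script fills RoidArray with static mesh asteroids between MinDistance and MaxDistance.
; BeginPlay destroys them and adds destructible components with newly randomized transforms, using hard-coded scale ranges instead of MaxScale and ScaleMultiplier.
; If HasTarget is set, it also spawns a TargetPoint at the actor's location.
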(event EventBeginPlay
  (Utilities|FlowControl|Sequence
    (:then_0
      (for _array_element (Variables|Default|GetRoidArray)
        (Components|DestroyComponent _array_element))
      (for _index (range 1 (Variables|AsteroidProperties|GetTotalRoids))
        (AddComponent|AddDestructibleComponent false (Math|Transform|MakeTransform (* (Math|Random|RandomUnitVector) (Math|Random|RandomFloatinRange (Variables|AsteroidProperties|GetMinDistance) (Variables|AsteroidProperties|GetMaxDistance))) (Math|Random|RandomRotator false) (Math|Conversions|ToVector(Float) (* (Math|Random|RandomFloatinRange 1.0 (Math|Random|RandomFloatinRange 1.0 15.0)) (Math|Random|RandomFloatinRange 0.5 1.2)))))))
    (:then_1
      (if (Variables|Default|GetHasTarget)
        (Game|SpawnActorfromClass "/Script/Engine.TargetPoint" (Math|Transform|MakeTransform (Transformation|GetActorLocation)) "Undefined" 0 0)))))

(fn ConstructionScript
  (for _index (range 1 (Variables|AsteroidProperties|GetTotalRoids))
    (bind _returnvalue (AddComponent|AddStaticMeshComponent false (Math|Transform|MakeTransform (* (Math|Random|RandomUnitVector) (Math|Random|RandomFloatinRange (Variables|AsteroidProperties|GetMinDistance) (Variables|AsteroidProperties|GetMaxDistance))) (Math|Random|RandomRotator false) (Math|Conversions|ToVector(Float) (* (Math|Random|RandomFloatinRange 1.0 (Variables|AsteroidProperties|GetMaxScale)) (Variables|AsteroidProperties|GetScaleMultiplier))))))
    (Utilities|Array|Add (Variables|Default|GetRoidArray) _returnvalue)))